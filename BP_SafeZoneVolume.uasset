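; BP_SafeZoneVolume is a box volume that makes overlapping actors immune to damage.
; Begin overlap on the Box clears the other actor's CanBeDamaged flag.
; End overlap sets it back to true only once the volume no longer overlaps that actor at all, rather than restoring its previous value.
; The construction script applies the BoxExtent and Hidden variables to the Box's size and in-game visibility.
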(event `self.Box.OnComponentBeginOverlap`
  (params (OverlappedComponent :type "PrimitiveComponent Object Reference") (OtherActor :type "Actor Object Reference") (OtherComp :type "PrimitiveComponent Object Reference") (OtherBodyIndex :type Integer) (bFromSweep :type Boolean) (SweepResult :type "HitResult Structure (by ref)"))
  (set `Actor.bCanBeDamaged` false OtherActor))

(event `self.Box.OnComponentEndOverlap`
  (params (OverlappedComponent :type "PrimitiveComponent Object Reference") (OtherActor :type "Actor Object Reference") (OtherComp :type "PrimitiveComponent Object Reference") (OtherBodyIndex :type Integer))
  (if (not (`self.IsOverlappingActor` self OtherActor))
    (set `Actor.bCanBeDamaged` true OtherActor)))

(fn `UserConstructionScript`
  (`BoxComponent.SetBoxExtent` (`self.Box`) (`self.BoxExtent`) true)
  (`SceneComponent.SetHiddenInGame` (`self.Box`) (`self.Hidden`) false))